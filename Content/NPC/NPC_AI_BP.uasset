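; NPC AI controller that runs the Patrol behavior tree on the PatrolData blackboard when play begins.
; GetWaypoint casts the controlled pawn to ThirdPersonCharacter and writes its first patrol point, always index 0, to the Waypoint blackboard key.
; AI perception updates only log the pawn name, sense class and perceived actor, with on-screen printing off; they do not affect the blackboard.
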(event `self.ReceiveBeginPlay`
  (`self.UseBlackboard` "/Game/NPC/PatrolData.PatrolData")
  (`self.RunBehaviorTree` "/Game/NPC/Patrol.Patrol"))

(event `self.AIPerception.OnTargetPerceptionUpdated`
  (params (Actor :type "Actor Object Reference") (Stimulus :type "AIStimulus Structure"))
  (bind _returnvalue (`AIPerceptionSystem.GetSenseClassForStimulus` Stimulus))
  (`KismetSystemLibrary.PrintString` (`KismetStringLibrary.Concat_StrStr` (`KismetSystemLibrary.GetObjectName` (`self.K2_GetPawn`)) " " (`KismetSystemLibrary.GetClassDisplayName` _returnvalue) ": " (`KismetSystemLibrary.GetObjectName` Actor)) false))

(fn `GetWaypoint`
  (params (Blackboard :type "BlackboardComponent Object Reference"))
  (bind _asthird_person_character (cast `/Game/TRASH/ThirdPersonCharacter` (`self.K2_GetPawn`)))
  (`BlackboardComponent.SetValueAsObject` Blackboard "Waypoint" (`|GetArrayItem` (`/Game/TRASH/ThirdPersonCharacter.PatrolPoints` _asthird_person_character))))

(fn `UserConstructionScript`)