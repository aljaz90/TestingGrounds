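; AI controller for guard NPCs that starts the Guard behavior tree with the PatrolData blackboard on BeginPlay.
; AI Perception writes sensed actors without the "Enemy" tag to the blackboard's enemy key and clears it when such an actor is lost.
; Every tick, it switches the controlled character's Aiming and Shooting flags on whenever the controller has a valid focus actor, and off otherwise.
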(event `self.ReceiveBeginPlay`
  (bind _blackboardcomponent (`self.UseBlackboard` "/Game/Character/AI/PatrolData.PatrolData"))
  (`self.RunBehaviorTree` "/Game/Character/AI/Guard.Guard")
  (set `self.BlcakboardComp` _blackboardcomponent))

(event `self.AIPerception.OnTargetPerceptionUpdated`
  (params (Actor :type "Actor Object Reference") (Stimulus :type "AIStimulus Structure"))
  (bind _blcakboardcomp (`self.BlcakboardComp`))
  (bind _enemykey (`self.EnemyKey`))
  (if (`self.ActorHasTag` Actor "Enemy")
    _
    (elif (`.bSuccessfullySensed` (break `AIStimulus` Stimulus))
      (`BlackboardComponent.SetValueAsObject` _blcakboardcomp _enemykey Actor)
      (else
        (`BlackboardComponent.ClearValue` _blcakboardcomp _enemykey)))))

(event `self.ReceiveTick`
  (params (DeltaSeconds :type "Float (single-precision)"))
  (bind _returnvalue (`KismetSystemLibrary.IsValid` (`self.GetFocusActor`)))
  (bind _ascharacter (cast `/Game/Character/Behaviour/Character` (`self.K2_GetPawn`)))
  (set `/Game/Character/Behaviour/Character.Aiming` _returnvalue _ascharacter)
  (set `/Game/Character/Behaviour/Character.Shooting` _returnvalue _ascharacter))

(fn `UserConstructionScript`)