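; Sci-fi door actor that opens when the player enters its sphere trigger, or on a key event, unless locked.
; Chained timelines slide optional front locks, front panels, then back panels, whose locks follow past a threshold.
; Leaving the trigger reverses the sequence after a delay unless KeepOpen is set.
; The construction script applies materials and user-set hue, light intensity and lock-state colors to every mesh.
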(event `self.sphere_collision_trigger.OnComponentBeginOverlap`
  (params (OverlappedComponent :type "PrimitiveComponent Object Reference") (OtherActor :type "Actor Object Reference") (OtherComp :type "PrimitiveComponent Object Reference") (OtherBodyIndex :type Integer) (bFromSweep :type Boolean) (SweepResult :type "HitResult Structure (by ref)"))
  (bind _posclosed (`self.posClosed`))
  (bind _posclosed_2 (`self.posClosed`))
  (bind _minusone (`self.minusOne`))
  ;[1 1 1] Verify that the player enter in the trigger
  (if (== OtherActor (`GameplayStatics.GetPlayerPawn` 0))
    ;[1 1 1] Verify if the door has to kept closed and if the user has to press a key to open
    (if (not (`self.isLock`))
      (set `self.isInCollision` true)
      (if (not (`self.useKeyToOpen`))
        ;[1 1 1] Verify if the door is already open
        (if (not (`self.isOpen`)) :!label _label
          ;[1 1 1] Execute the animation that Open the door
          (if (`self.animateLocks`)
            (`TimelineComponent.SetPlayRate` (`self.OpenLocks`) (/ 1.0 (`self.TimeSegLocksAnimation`)))
            (bind (_direction _openscalar) (`Timeline|OpenLocks` :!via `PlayFromStart`)
              (:`Update`
                (bind _returnvalue (`KismetMathLibrary.Lerp` 0.0 10.0 _openscalar))
                (`SceneComponent.K2_SetRelativeLocation` (`self.door05FrontRightLock_1`) (`KismetMathLibrary.MakeVector` _returnvalue) false false)
                (`SceneComponent.K2_SetRelativeLocation` (`self.door05FrontLeftLock_2`) (`KismetMathLibrary.MakeVector` _returnvalue) false false)
                (`SceneComponent.K2_SetRelativeLocation` (`self.door05FrontLeftLock_1`) (`KismetMathLibrary.MakeVector` (* _returnvalue (`self.minusOne`))) false false)
                (`SceneComponent.K2_SetRelativeLocation` (`self.door05FrontRightLock_2`) (`KismetMathLibrary.MakeVector` (* _returnvalue (`self.minusOne`))) false false))
              (:`Finished`
                (`KismetSystemLibrary.Delay` 0.5)
                (`TimelineComponent.SetPlayRate` (`self.OpenDoorFront`) (/ 1.0 (`self.TimeSegOpenDoor`)) :!label _label_2)
                (bind (_direction_2 _openscalar_2) (`Timeline|OpenDoorFront` :!via `PlayFromStart`)
                  (:`Update`
                    (`SceneComponent.K2_SetRelativeLocation` (`self.door05Frontright`) (`KismetMathLibrary.MakeVector` (`KismetMathLibrary.Lerp` _posclosed (`self.posOpen_Frontright`) _openscalar_2)) false false)
                    (`SceneComponent.K2_SetRelativeLocation` (`self.door05Frontleft`) (`KismetMathLibrary.MakeVector` (* (`KismetMathLibrary.Lerp` _posclosed (`self.posOpen_Frontleft`) _openscalar_2) (`self.minusOne`))) false false))
                  (:`Finished`
                    (`KismetSystemLibrary.Delay` 0.5)
                    (`TimelineComponent.SetPlayRate` (`self.OpenDoorBack`) (/ 1.0 (`self.TimeSegOpenDoor`)))
                    (bind (_direction_3 _openscalar_3) (`Timeline|OpenDoorBack` :!via `PlayFromStart`)
                      (:`Update`
                        (bind _returnvalue_2 (`KismetMathLibrary.Lerp` _posclosed_2 (`self.posOpen_BackTop`) _openscalar_3))
                        (`SceneComponent.K2_SetRelativeLocation` (`self.door05BackTop`) (`KismetMathLibrary.MakeVector` 0.0 0.0 _returnvalue_2) false false)
                        (bind _returnvalue_3 (`KismetMathLibrary.Lerp` _posclosed_2 (`self.posOpen_BackDown`) _openscalar_3))
                        (`SceneComponent.K2_SetRelativeLocation` (`self.door05BackDown`) (`KismetMathLibrary.MakeVector` 0.0 0.0 (* _returnvalue_3 _minusone)) false false)
                        (`|ExecutionSequence`
                          (:`then_0`
                            (if (>= _returnvalue_2 17.0)
                              (`SceneComponent.K2_SetRelativeLocation` (`self.door05BackTopLock`) (`KismetMathLibrary.MakeVector` 0.0 0.0 (- _returnvalue_2 17.0)) false false)))
                          (:`then_1`
                            (if (>= _returnvalue_3 17.0)
                              (`SceneComponent.K2_SetRelativeLocation` (`self.door05BackDownLock`) (`KismetMathLibrary.MakeVector` 0.0 0.0 (* (- _returnvalue_3 17.0) _minusone)) false false)))
                          (:`then_2`
                            (set `self.isOpen` true)))))))))
            (else
              (goto _label_2))))))))

(event `/Game/DoorSciFi_Pack02/Blueprints/BPI_Doors.pressOpenKey`
  ;[1 1 1] Press the Open key and verify status to determine if is possible to open the door
  (if (`self.isLock`)
    _
    (elif (`self.useKeyToOpen`)
      (if (`self.isInCollision`)
        (goto _label)))))

(event `self.sphere_collision_trigger.OnComponentEndOverlap`
  (params (OverlappedComponent :type "PrimitiveComponent Object Reference") (OtherActor :type "Actor Object Reference") (OtherComp :type "PrimitiveComponent Object Reference") (OtherBodyIndex :type Integer))
  (bind _posclosed (`self.posClosed`))
  (bind _door05backdownlock (`self.door05BackDownLock`))
  (bind _door05backtoplock (`self.door05BackTopLock`))
  (bind _posclosed_2 (`self.posClosed`))
  (bind _minusone (`self.minusOne`))
  ;[1 1 1] Verify that the player leave the trigger
  (if (== OtherActor (`GameplayStatics.GetPlayerPawn` 0))
    ;[1 1 1] Verify if the door has to kept closed and if the door has to kept open
    (if (not (`self.isLock`))
      (set `self.isInCollision` false)
      (if (not (`self.keepOpen`))
        ;[1 1 1] Verified if the door is open and wait one second to close it
        (if (`self.isOpen`)
          (`KismetSystemLibrary.Delay` 1.0)
          ;[1 1 1] Execute the animation that close the door
          (`TimelineComponent.SetPlayRate` (`self.CloseDoorBack`) (/ 1.0 (`self.TimeSegOpenDoor`)))
          (bind (_direction _openscalar) (`Timeline|CloseDoorBack` :!via `ReverseFromEnd`)
            (:`Update`
              (bind _returnvalue (`KismetMathLibrary.Lerp` _posclosed_2 (`self.posOpen_BackTop`) _openscalar))
              (`SceneComponent.K2_SetRelativeLocation` (`self.door05BackTop`) (`KismetMathLibrary.MakeVector` 0.0 0.0 _returnvalue) false false)
              (bind _returnvalue_2 (`KismetMathLibrary.Lerp` _posclosed_2 (`self.posOpen_BackDown`) _openscalar))
              (`SceneComponent.K2_SetRelativeLocation` (`self.door05BackDown`) (`KismetMathLibrary.MakeVector` 0.0 0.0 (* _returnvalue_2 _minusone)) false false)
              (`|ExecutionSequence`
                (:`then_0`
                  (if (>= _returnvalue 17.0)
                    (`SceneComponent.K2_SetRelativeLocation` _door05backtoplock (`KismetMathLibrary.MakeVector` 0.0 0.0 (- _returnvalue 17.0)) false false)
                    (else
                      (`SceneComponent.K2_SetRelativeLocation` _door05backtoplock (0.0 0.0 0.0) false false))))
                (:`then_1`
                  (if (>= _returnvalue_2 17.0)
                    (`SceneComponent.K2_SetRelativeLocation` _door05backdownlock (`KismetMathLibrary.MakeVector` 0.0 0.0 (* (- _returnvalue_2 17.0) _minusone)) false false)
                    (else
                      (`SceneComponent.K2_SetRelativeLocation` _door05backdownlock (0.0 0.0 0.0) false false))))))
            (:`Finished`
              (`KismetSystemLibrary.Delay` 0.5)
              (`TimelineComponent.SetPlayRate` (`self.CloseDoorFront`) (/ 1.0 (`self.TimeSegOpenDoor`)))
              (bind (_direction_2 _openscalar_2) (`Timeline|CloseDoorFront` :!via `ReverseFromEnd`)
                (:`Update`
                  (`SceneComponent.K2_SetRelativeLocation` (`self.door05Frontright`) (`KismetMathLibrary.MakeVector` (`KismetMathLibrary.Lerp` _posclosed (`self.posOpen_Frontright`) _openscalar_2)) false false)
                  (`SceneComponent.K2_SetRelativeLocation` (`self.door05Frontleft`) (`KismetMathLibrary.MakeVector` (* (`KismetMathLibrary.Lerp` _posclosed (`self.posOpen_Frontleft`) _openscalar_2) (`self.minusOne`))) false false)
                  (set `self.isOpen` false))
                (:`Finished`
                  (`KismetSystemLibrary.Delay` 0.5)
                  (if (`self.animateLocks`)
                    (`TimelineComponent.SetPlayRate` (`self.CloseLocks`) (/ 1.0 (`self.TimeSegLocksAnimation`)))
                    (bind (_direction_3 _openscalar_3) (`Timeline|CloseLocks` :!via `ReverseFromEnd`)
                      (:`Update`
                        (bind _returnvalue_3 (`KismetMathLibrary.Lerp` 0.0 10.0 _openscalar_3))
                        (`SceneComponent.K2_SetRelativeLocation` (`self.door05FrontRightLock_1`) (`KismetMathLibrary.MakeVector` _returnvalue_3) false false)
                        (`SceneComponent.K2_SetRelativeLocation` (`self.door05FrontLeftLock_2`) (`KismetMathLibrary.MakeVector` _returnvalue_3) false false)
                        (`SceneComponent.K2_SetRelativeLocation` (`self.door05FrontLeftLock_1`) (`KismetMathLibrary.MakeVector` (* _returnvalue_3 (`self.minusOne`))) false false)
                        (`SceneComponent.K2_SetRelativeLocation` (`self.door05FrontRightLock_2`) (`KismetMathLibrary.MakeVector` (* _returnvalue_3 (`self.minusOne`))) false false)))))))))))))

(fn `UserConstructionScript`
  (bind _hueshift (`self.HueShift`))
  (bind _intensitydoorlight (`self.IntensityDoorLight`))
  (bind _materialsparametersname (`self.materialsParametersName`))
  (bind _staticmeshdoorback (`self.staticmeshDoorBack`))
  (bind _islock (`self.isLock`))
  (bind _door05frame (`self.door05frame`))
  (bind _staticmeshdoorfront (`self.staticmeshDoorFront`))
  (bind _returnvalue (`KismetMathLibrary.Conv_LinearColorToVector` (`self.ColorLightDoorGeneral`)))
  (bind _returnvalue_2 (`KismetMathLibrary.Conv_LinearColorToVector` (`self.ColorLightLock`)))
  (bind _returnvalue_3 (`KismetMathLibrary.Conv_LinearColorToVector` (`self.ColorLightUnlock`)))
  (bind _output (`|GetArrayItem` _materialsparametersname))
  (bind _output_2 (`|GetArrayItem` _materialsparametersname 1))
  (bind _output_3 (`|GetArrayItem` _materialsparametersname 2))
  (bind _output_4 (`|GetArrayItem` _materialsparametersname 3))
  (bind _output_5 (`|GetArrayItem` _materialsparametersname 4))
  ;[1 1 1] Set the material on each static mesh
  (set `self.staticmeshDoorFront` (`|MakeArray` (`self.door05FrontRightLock_2`) (`self.door05Frontright`) (`self.door05Frontleft`) (`self.door05FrontRightLock_1`) (`self.door05FrontLeftLock_1`) (`self.door05FrontLeftLock_2`)))
  (set `self.staticmeshDoorBack` (`|MakeArray` (`self.door05BackTopLock`) (`self.door05BackDownLock`) (`self.door05BackDown`) (`self.door05BackTop`)))
  (`PrimitiveComponent.SetMaterial` (`self.door05frame`) 0 (`self.Mframe`))
  (for _array_element _staticmeshdoorfront
    (`PrimitiveComponent.SetMaterial` _array_element 0 (`self.Mdoorfront`)))
  (for _array_element_2 _staticmeshdoorback
    (`PrimitiveComponent.SetMaterial` _array_element_2 0 (`self.Mdoorback`)))
  ;[1 1 1] Set the parameters on each materials that the user modified in the blueprint
  (`|ExecutionSequence`
    (:`then_0`
      (`MeshComponent.SetScalarParameterValueOnMaterials` _door05frame _output _hueshift)
      (`MeshComponent.SetScalarParameterValueOnMaterials` _door05frame _output_2 _intensitydoorlight)
      (`MeshComponent.SetScalarParameterValueOnMaterials` _door05frame _output_3 _intensitydoorlight)
      (`MeshComponent.SetVectorParameterValueOnMaterials` _door05frame _output_4 _returnvalue)
      (if _islock
        (`MeshComponent.SetVectorParameterValueOnMaterials` _door05frame _output_5 _returnvalue_2)
        (else
          (`MeshComponent.SetVectorParameterValueOnMaterials` _door05frame _output_5 _returnvalue_3))))
    (:`then_1`
      (for _array_element_3 _staticmeshdoorfront
        (`MeshComponent.SetScalarParameterValueOnMaterials` _array_element_3 _output _hueshift)
        (`MeshComponent.SetScalarParameterValueOnMaterials` _array_element_3 _output_2 _intensitydoorlight)
        (`MeshComponent.SetScalarParameterValueOnMaterials` _array_element_3 _output_3 _intensitydoorlight)
        (`MeshComponent.SetVectorParameterValueOnMaterials` _array_element_3 _output_4 _returnvalue)
        (if _islock
          (`MeshComponent.SetVectorParameterValueOnMaterials` _array_element_3 _output_5 _returnvalue_2)
          (else
            (`MeshComponent.SetVectorParameterValueOnMaterials` _array_element_3 _output_5 _returnvalue_3)))))
    (:`then_2`
      (for _array_element_4 _staticmeshdoorback
        (`MeshComponent.SetScalarParameterValueOnMaterials` _array_element_4 _output _hueshift)
        (`MeshComponent.SetScalarParameterValueOnMaterials` _array_element_4 _output_2 _intensitydoorlight)
        (`MeshComponent.SetScalarParameterValueOnMaterials` _array_element_4 _output_3 _intensitydoorlight)
        (`MeshComponent.SetVectorParameterValueOnMaterials` _array_element_4 _output_4 _returnvalue)
        (if _islock
          (`MeshComponent.SetVectorParameterValueOnMaterials` _array_element_4 _output_5 _returnvalue_2)
          (else
            (`MeshComponent.SetVectorParameterValueOnMaterials` _array_element_4 _output_5 _returnvalue_3)))))))