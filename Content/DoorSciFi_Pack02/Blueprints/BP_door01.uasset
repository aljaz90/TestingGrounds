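; Sci-fi sliding door that opens for player pawn 0 on entering a sphere trigger, or on a key press inside it, unless locked.
; Timelines slide the upper and lower panels apart, with the lower lock piece trailing past a threshold.
; Leaving the trigger closes it after a one-second delay unless KeepOpen is set.
; The construction script applies materials, hue, light intensity and lock-state colors to frame and panels.
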(event `self.sphere_collision_trigger.OnComponentBeginOverlap`
  (params (OverlappedComponent :type "PrimitiveComponent Object Reference") (OtherActor :type "Actor Object Reference") (OtherComp :type "PrimitiveComponent Object Reference") (OtherBodyIndex :type Integer) (bFromSweep :type Boolean) (SweepResult :type "HitResult Structure (by ref)"))
  (bind _posclosed (`self.posClosed`))
  (bind _minusone (`self.minusOne`))
  ;[1 1 1] Verify that the player enter in the trigger
  (if (== OtherActor (`GameplayStatics.GetPlayerPawn` 0))
    ;[1 1 1] Verify if the door has to kept closed and if the user has to press a key to open
    (if (not (`self.isLock`))
      (set `self.isInCollision` true)
      (if (not (`self.useKeyToOpen`))
        ;[1 1 1] Verify if the door is already open
        (if (not (`self.isOpen`)) :!label _label
          ;[1 1 1] Execute the animation that Open the door
          (`TimelineComponent.SetPlayRate` (`self.OpenDoor`) (/ 1.0 (`self.TimeSegOpenDoor`)))
          (bind (_direction _openscalar) (`Timeline|OpenDoor` :!via `PlayFromStart`)
            (:`Update`
              (`SceneComponent.K2_SetRelativeLocation` (`self.door01up`) (`KismetMathLibrary.MakeVector` 0.0 0.0 (`KismetMathLibrary.Lerp` _posclosed (`self.posOpen_up`) _openscalar)) false false)
              (bind _returnvalue (`KismetMathLibrary.Lerp` _posclosed (`self.posOpen_down`) _openscalar))
              (`SceneComponent.K2_SetRelativeLocation` (`self.door01down`) (`KismetMathLibrary.MakeVector` 0.0 0.0 (* _returnvalue _minusone)) false false)
              (if (>= _returnvalue 18.0)
                (`SceneComponent.K2_SetRelativeLocation` (`self.door01lockdown`) (`KismetMathLibrary.MakeVector` 0.0 0.0 (* (- _returnvalue 18.0) _minusone)) false false)
                (set `self.isOpen` true)))))))))

(event `/Game/DoorSciFi_Pack02/Blueprints/BPI_Doors.pressOpenKey`
  ;[1 1 1] Press the Open key and verify status to determine if is possible to open the door
  (if (`self.isLock`)
    _
    (elif (`self.useKeyToOpen`)
      (if (`self.isInCollision`)
        (goto _label)))))

(event `self.sphere_collision_trigger.OnComponentEndOverlap`
  (params (OverlappedComponent :type "PrimitiveComponent Object Reference") (OtherActor :type "Actor Object Reference") (OtherComp :type "PrimitiveComponent Object Reference") (OtherBodyIndex :type Integer))
  (bind _posclosed (`self.posClosed`))
  (bind _minusone (`self.minusOne`))
  ;[1 1 1] Verify that the player leave the trigger
  (if (== OtherActor (`GameplayStatics.GetPlayerPawn` 0))
    ;[1 1 1] Verify if the door has to kept closed and if the door has to kept open
    (if (not (`self.isLock`))
      (set `self.isInCollision` false)
      (if (not (`self.keepOpen`))
        ;[1 1 1] Verified if the door is open and wait one second to close it
        (if (`self.isOpen`)
          (`KismetSystemLibrary.Delay` 1.0)
          ;[1 1 1] Execute the animation that close the door
          (`TimelineComponent.SetPlayRate` (`self.CloseDoor`) (/ 1.0 (`self.TimeSegOpenDoor`)))
          (bind (_direction _openscalar) (`Timeline|CloseDoor` :!via `ReverseFromEnd`)
            (:`Update`
              (`SceneComponent.K2_SetRelativeLocation` (`self.door01up`) (`KismetMathLibrary.MakeVector` 0.0 0.0 (`KismetMathLibrary.Lerp` _posclosed (`self.posOpen_up`) _openscalar)) false false)
              (bind _returnvalue (`KismetMathLibrary.Lerp` _posclosed (`self.posOpen_down`) _openscalar))
              (`SceneComponent.K2_SetRelativeLocation` (`self.door01down`) (`KismetMathLibrary.MakeVector` 0.0 0.0 (* _returnvalue _minusone)) false false)
              (if (>= _returnvalue 18.0)
                (`SceneComponent.K2_SetRelativeLocation` (`self.door01lockdown`) (`KismetMathLibrary.MakeVector` 0.0 0.0 (* (- _returnvalue 18.0) _minusone)) false false)
                (set `self.isOpen` false)))))))))

(fn `UserConstructionScript`
  (bind _hueshift (`self.HueShift`))
  (bind _intensitydoorlight (`self.IntensityDoorLight`))
  (bind _materialsparametersname (`self.materialsParametersName`))
  (bind _islock (`self.isLock`))
  (bind _door01frame (`self.door01frame`))
  (bind _staticmeshdoor (`self.staticmeshDoor`))
  (bind _returnvalue (`KismetMathLibrary.Conv_LinearColorToVector` (`self.ColorLightDoorGeneral`)))
  (bind _returnvalue_2 (`KismetMathLibrary.Conv_LinearColorToVector` (`self.ColorLightLock`)))
  (bind _returnvalue_3 (`KismetMathLibrary.Conv_LinearColorToVector` (`self.ColorLightUnlock`)))
  (bind _output (`|GetArrayItem` _materialsparametersname))
  (bind _output_2 (`|GetArrayItem` _materialsparametersname 1))
  (bind _output_3 (`|GetArrayItem` _materialsparametersname 2))
  (bind _output_4 (`|GetArrayItem` _materialsparametersname 3))
  (bind _output_5 (`|GetArrayItem` _materialsparametersname 4))
  ;[1 1 1] Set the material on each static mesh
  (set `self.staticmeshDoor` (`|MakeArray` (`self.door01lockdown`) (`self.door01down`) (`self.door01up`)))
  (`PrimitiveComponent.SetMaterial` (`self.door01frame`) 0 (`self.Mframe`))
  (for _array_element _staticmeshdoor
    (`PrimitiveComponent.SetMaterial` _array_element 0 (`self.Mdoor`)))
  ;[1 1 1] Set the parameters on each materials that the user modified in the blueprint
  (`|ExecutionSequence`
    (:`then_0`
      (`MeshComponent.SetScalarParameterValueOnMaterials` _door01frame _output _hueshift)
      (`MeshComponent.SetScalarParameterValueOnMaterials` _door01frame _output_2 _intensitydoorlight)
      (`MeshComponent.SetScalarParameterValueOnMaterials` _door01frame _output_3 _intensitydoorlight)
      (`MeshComponent.SetVectorParameterValueOnMaterials` _door01frame _output_4 _returnvalue)
      (if _islock
        (`MeshComponent.SetVectorParameterValueOnMaterials` _door01frame _output_5 _returnvalue_2)
        (else
          (`MeshComponent.SetVectorParameterValueOnMaterials` _door01frame _output_5 _returnvalue_3))))
    (:`then_1`
      (for _array_element_2 _staticmeshdoor
        (`MeshComponent.SetScalarParameterValueOnMaterials` _array_element_2 _output _hueshift)
        (`MeshComponent.SetScalarParameterValueOnMaterials` _array_element_2 _output_2 _intensitydoorlight)
        (`MeshComponent.SetScalarParameterValueOnMaterials` _array_element_2 _output_3 _intensitydoorlight)
        (`MeshComponent.SetVectorParameterValueOnMaterials` _array_element_2 _output_4 _returnvalue)
        (if _islock
          (`MeshComponent.SetVectorParameterValueOnMaterials` _array_element_2 _output_5 _returnvalue_2)
          (else
            (`MeshComponent.SetVectorParameterValueOnMaterials` _array_element_2 _output_5 _returnvalue_3)))))))